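; Spectator pawn that serves as a player's placeholder until they pick a class to spawn as.
; An assigned index opens ClassSelectMenu with UI-only input and cursor, passing the index along; a locally controlled pawn with authority assigns itself index 0 on BeginPlay.
; SpawnAsClass spawns the given class at the pawn's transform, has the controller possess it, derives team from index divided by two, then destroys the spectator.
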(event `SpawnAsClass`
  (params (Class :type "/Game/Character/Blueprints/PlayerBase Class Reference") (Index :type Integer))
  (bind _returnvalue (`self.GetController`))
  (bind _returnvalue_2 (`|SpawnActorFromClass` Class (`self.GetTransform`) "Undefined" "OverrideRootScale" _returnvalue))
  (`Controller.Possess` _returnvalue _returnvalue_2)
  (`/Game/Character/Blueprints/PlayerBase.SetTeam` _returnvalue_2 (/ Index 2))
  (`self.K2_DestroyActor`))

(event `AssignIndex`
  (params (Index :type Integer))
  (`KismetSystemLibrary.PrintString` "Hello")
  (`self.AssignIndexLocal` Index))

(event `self.ReceiveBeginPlay`
  (`/Engine/EditorBlueprintResources/ActorMacros.Switch Has Authority`
    (:`Authority`
      (if (`self.IsLocallyControlled`)
        (`self.AssignIndexLocal` 0)))))

(fn `AssignIndexLocal`
  (params (Index :type Integer))
  (bind _returnvalue (`Controller.CastToPlayerController` (`self.GetController`)))
  (bind _returnvalue_2 (`|CreateWidget` "/Game/Game/Menus/ClassSelectMenu.ClassSelectMenu_C" _returnvalue))
  (`UserWidget.AddToViewport` _returnvalue_2 1)
  (`WidgetBlueprintLibrary.SetInputMode_UIOnlyEx` _returnvalue _returnvalue_2)
  (`/Game/Game/Menus/ClassSelectMenu.AssignSpawnIndex` _returnvalue_2 Index)
  (set `PlayerController.bShowMouseCursor` true _returnvalue)
  (return))

(fn `UserConstructionScript`)