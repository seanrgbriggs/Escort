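; Scout2 is a character Blueprint that adds a scoping ability for marking players on opposing teams.
; Holding Attack2 narrows the camera field of view and enables scouting, and releasing it restores the wider view.
; While scouting, Tick runs a long camera raycast each frame and refreshes TagTime on any hit PlayerBase from another team.
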(event `self.ReceiveTick`
  (params (DeltaSeconds :type "Float (single-precision)"))
  (`parent.ReceiveTick` DeltaSeconds)
  (if (`self.Scouting`)
    (bind (_success _hit) (`self.RaycastFunc` (`self.Camera`) 100000.0))
    (if _success
      (bind _asplayer_base (cast `/Game/Character/Blueprints/PlayerBase` (`.HitActor` (`GameplayStatics.BreakHitResult` _hit))))
      (if (!= (`/Game/Character/Blueprints/PlayerBase.Team` _asplayer_base) (`self.Team`))
        (set `/Game/Character/Blueprints/PlayerBase.TagTime` 10.0 _asplayer_base)))))

(event `InputAction|Attack2`
  (params (Key :type "Key Structure" :default "AnyKey"))
  (bind _camera (`self.Camera`))
  (:`Pressed`
    (set `CameraComponent.FieldOfView` 50.0 _camera)
    (set `self.Scouting` true))
  (:`Released`
    (set `CameraComponent.FieldOfView` 90.0 _camera)
    (set `self.Scouting` false)))

(fn `UserConstructionScript`
  (`parent.UserConstructionScript`))