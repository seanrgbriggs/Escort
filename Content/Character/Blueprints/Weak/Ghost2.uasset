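; Ghost2 is a character Blueprint that cloaks while standing still and uncloaks when it moves.
; Tick checks for zero velocity and calls CloakEvent only when the Cloaked state needs to change.
; Cloaking caches the Mesh materials once, applies M_Cloak to Mesh and MeshFP, and disables the Mesh shadow.
; Uncloaking restores the shadow and applies the cached Mesh materials to both meshes, as MeshFP's own materials are never stored.
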(event `CloakEvent`
  (params (Hm :type Boolean))
  (if Hm
    (`self.Cloak`)
    (else
      (`self.Uncloak`))))

(event `Cloak`
  (bind _mesh (`self.Mesh`))
  (`self.StoreMaterials`)
  (`self.SetMaterials` _mesh)
  (`PrimitiveComponent.SetCastShadow` _mesh false)
  (`self.SetMaterials` (`self.Mesh_FP`))
  (set `self.Cloaked` true))

(event `Uncloak`
  (bind _mesh (`self.Mesh`))
  (`self.RestoreMaterials` _mesh)
  (`PrimitiveComponent.SetCastShadow` _mesh true)
  (`self.RestoreMaterials` (`self.Mesh_FP`))
  (set `self.Cloaked` false))

(event `InputAction|Attack2`
  (params (Key :type "Key Structure" :default "AnyKey")))

(event `self.ReceiveTick`
  (params (DeltaSeconds :type "Float (single-precision)"))
  (bind _cloaked (`self.Cloaked`))
  (`parent.ReceiveTick` DeltaSeconds)
  (if (== (`KismetMathLibrary.VSizeSquared` (`self.GetVelocity`)) 0.0)
    (if (not _cloaked)
      (`self.CloakEvent` true))
    (elif _cloaked
      (`self.CloakEvent` false))))

(fn `RestoreMaterials`
  (params (Component :type "PrimitiveComponent Object Reference"))
  (bind _materialstorage (`self.MaterialStorage`))
  (for _index (range (`KismetArrayLibrary.Array_Length` _materialstorage))
    (`PrimitiveComponent.SetMaterial` Component _index (`KismetArrayLibrary.Array_Get` _materialstorage _index))))

(fn `SetMaterials`
  (params (Comonent :type "MeshComponent Object Reference"))
  (for _index (range (`KismetArrayLibrary.Array_Length` (`MeshComponent.GetMaterials` Comonent)))
    (`PrimitiveComponent.SetMaterial` Comonent _index "/Game/Materials/M_Cloak.M_Cloak")))

(fn `StoreMaterials`
  (bind _materialstorage (`self.MaterialStorage`))
  (bind _mesh (`self.Mesh`))
  (if (== 0 (`KismetArrayLibrary.Array_Length` _materialstorage))
    (for _index (range (`PrimitiveComponent.GetNumMaterials` _mesh))
      (`KismetArrayLibrary.Array_Add` _materialstorage (`PrimitiveComponent.GetMaterial` _mesh _index)))))

(fn `UserConstructionScript`
  (`parent.UserConstructionScript`))