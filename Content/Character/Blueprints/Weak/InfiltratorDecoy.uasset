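; InfiltratorDecoy is a controllable decoy for the Infiltrator character that a player can dismiss.
; Pressing Attack2 calls Despawn, which has the decoy's controller possess the stored Parent pawn and then destroys the decoy.
; All other graph events and the construction script only defer to the parent class or do nothing.
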(event `self.ReceiveBeginPlay`
  (`parent.ReceiveBeginPlay`))

(event `self.ReceiveActorBeginOverlap`
  (params (OtherActor :type "Actor Object Reference")))

(event `self.ReceiveTick`
  (params (DeltaSeconds :type "Float (single-precision)"))
  (`parent.ReceiveTick` 0.0))

(event `Despawn`
  (`Controller.Possess` (`self.GetController`) (`self.Parent`))
  (`self.K2_DestroyActor`))

(event `InputAction|Attack2`
  (params (Key :type "Key Structure" :default "AnyKey"))
  (:`Pressed`
    (`self.Despawn`)))

(fn `UserConstructionScript`
  (`parent.UserConstructionScript`))