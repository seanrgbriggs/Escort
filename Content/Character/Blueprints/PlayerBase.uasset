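; PlayerBase is the player character Blueprint, handling jump, movement and look input.
; Movement follows control yaw only, while look axes feed controller pitch and yaw.
; Each look update rebuilds the camera's relative rotation from the rotation cached at BeginPlay, applying negated control pitch as roll.
; Horizontal look input is also stored as TurnRate through a SetTurnRate event.
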(event `self.ReceiveBeginPlay`
  (set `self.CamRot` (`SceneComponent.RelativeRotation` (`self.Camera`))))

(event `InputAction|Jump`
  (params (Key :type "Key Structure" :default "AnyKey"))
  (:`Pressed`
    (`self.Jump`)))

(event `InputAxis|MoveForward`
  (params (AxisValue :type "Float (single-precision)"))
  (`self.AddMovementInput` (`KismetMathLibrary.GetForwardVector` (`KismetMathLibrary.MakeRotator` 0.0 0.0 (.yaw (`self.GetControlRotation`)))) AxisValue))

(event `InputAxis|MoveRight`
  (params (AxisValue :type "Float (single-precision)"))
  (`self.AddMovementInput` (`KismetMathLibrary.GetRightVector` (`KismetMathLibrary.MakeRotator` 0.0 0.0 (.yaw (`self.GetControlRotation`)))) AxisValue))

(event `InputAxis|LookUp`
  (params (AxisValue :type "Float (single-precision)"))
  (`self.AddControllerPitchInput` AxisValue)
  (`SceneComponent.K2_SetRelativeRotation` (`self.Camera`) (`KismetMathLibrary.ComposeRotators` (`self.CamRot`) (`KismetMathLibrary.MakeRotator` (* (.pitch (`self.GetControlRotation`)) -1.0))) false false :!label _label))

(event `InputAxis|LookRight`
  (params (AxisValue :type "Float (single-precision)"))
  (bind _output_get (set `self.TurnRate` AxisValue))
  (`self.AddControllerYawInput` _output_get)
  (`self.SetTurnRate` _output_get)
  (goto _label))

(event `SetTurnRate`
  (params (NewTurnRate :type "Float (double-precision)"))
  (set `self.TurnRate` NewTurnRate))

(fn `UserConstructionScript`)