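; Hunter is a strong-type character Blueprint that sets its leap angle on play and extends its parent's tick with claw effects.
; Left sparks run while grounded, right sparks while arms follow the camera, meaning neither wall-jumped nor climbing.
; While falling, a cone trace, fed zero start and direction vectors, debug-prints hits and spawns claw sparks on opposing-team players, without applying damage.
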(event `self.ReceiveBeginPlay`
  (set `self.Leap Angle` 345.0))

(event `self.ReceiveTick`
  (params (DeltaSeconds :type "Float (single-precision)"))
  (bind _returnvalue (`NavMovementComponent.IsFalling` (`self.CharacterMovement`)))
  (`parent.ReceiveTick` DeltaSeconds)
  (`ActorComponent.SetActive` (`self.SparksLeft`) (not _returnvalue) false)
  (`ActorComponent.SetActive` (`self.SparksRight`) (`self.ArmsFollowCamera`) false)
  (if _returnvalue
    (bind (_hit _success) (`self.ConeTraceLines` (0.0 0.0 0.0) (0.0 0.0 0.0)))
    (if _success
      (`KismetSystemLibrary.PrintString` "Hello" true true (struct :`G` 0.66 :`B` 1.0 :`A` 1.0) 20.0)
      (bind (_bblockinghit _binitialoverlap _time _location _impactpoint _normal _impactnormal _physmat _hitactor) (`GameplayStatics.BreakHitResult` _hit))
      (bind _asplayer_base (cast `/Game/Character/Blueprints/PlayerBase` _hitactor))
      (if (!= (`/Game/Character/Blueprints/PlayerBase.Team` _asplayer_base) (`self.Team`))
        (`GameplayStatics.SpawnEmitterAtLocation` "/Game/StarterContent/Particles/ClawSparks.ClawSparks" _location)))))

(fn `ArmsFollowCamera`
  (returns (Result :type Boolean))
  (return (`KismetMathLibrary.BooleanNOR` (`self.WallJumped`) (`self.IsClimbing`))))

(fn `UserConstructionScript`
  (`parent.UserConstructionScript`))