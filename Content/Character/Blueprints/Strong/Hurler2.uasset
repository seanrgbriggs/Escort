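; Hurler2 is a strong robot character that throws charged antimatter projectiles and can launch weaker teammates.
; Tick grows the Antimatter mesh toward a size cap, hiding it while falling and running MatterForm while charging on the ground.
; Attack1 at full charge sets a throw montage, then spawns an impulsed HurlerProjectile and resets the charge.
; Attack2 raycasts for a same-team WeakRobot2 on press and launches it along camera forward on release if nearby.
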(event `self.ReceiveTick`
  (params (DeltaSeconds :type "Float (single-precision)"))
  (bind _projectilesize (`self.ProjectileSize`))
  (bind _returnvalue (not (`NavMovementComponent.IsFalling` (`self.CharacterMovement`))))
  (`parent.ReceiveTick` DeltaSeconds)
  (`SceneComponent.SetRelativeScale3D` (`self.Antimatter`) (`KismetMathLibrary.MakeVector` _projectilesize _projectilesize _projectilesize))
  (set `self.ProjectileSize` (`KismetMathLibrary.FClamp` (+ _projectilesize (* DeltaSeconds 0.1)) 0.0 0.272))
  (`SceneComponent.SetVisibility` (`self.Antimatter`) _returnvalue false)
  (`ActorComponent.SetActive` (`self.MatterForm`) (and _returnvalue (< (`self.ProjectileSize`) 0.27)) false))

(event `ThrowServer`
  (bind _returnvalue (`SceneComponent.GetForwardVector` (`self.Camera`)))
  (if (> (`self.ProjectileSize`) 0.27)
    (set `self.PlayThisMontage` "/Game/Character/Animation/Strong/Hurler/hurler_throw_montage.hurler_throw_montage")
    (`KismetSystemLibrary.Delay` 1.0)
    (bind _returnvalue_2 (`|SpawnActorFromClass` "/Game/Props/Blueprints/HurlerProjectile.HurlerProjectile_C" (`KismetMathLibrary.MakeTransform` (+ (`SceneComponent.K2_GetComponentLocation` (`self.Antimatter`)) (* _returnvalue 100.0))) "AlwaysSpawn" "OverrideRootScale" (`self.GetController`)))
    (`PrimitiveComponent.AddImpulse` (`/Game/Props/Blueprints/HurlerProjectile.Sphere` _returnvalue_2) (* _returnvalue 4000.0) "None" true)
    (`self.Release`)
    (`KismetSystemLibrary.Delay` 1.0)
    (`self.Release`)))

(event `InputAction|Attack1`
  (params (Key :type "Key Structure" :default "AnyKey"))
  (:`Pressed`
    (`self.ThrowServer`)))

(event `Release`
  (set `self.ProjectileSize` 0.0))

(event `InputAction|Attack2`
  (params (Key :type "Key Structure" :default "AnyKey"))
  (:`Pressed`
    (`self.Throw Ally Server` true))
  (:`Released`
    (`self.Throw Ally Server` false)))

(event `Throw Ally Server`
  (params (Pressed :type Boolean))
  (bind _weakguy (`self.WeakGuy`))
  (if Pressed
    (bind (_success _hit) (`self.RaycastFunc` (`self.Camera`) 500.0))
    (if _success
      (bind _asweak_robot_2 (cast `/Game/Character/Blueprints/Weak/WeakRobot2` (`.HitActor` (`GameplayStatics.BreakHitResult` _hit))))
      (if (== (`self.Team`) (`/Game/Character/Blueprints/PlayerBase.Team` _asweak_robot_2))
        (set `self.HoldingAlly` true)
        (set `self.WeakGuy` _asweak_robot_2)))
    (elif (and (`self.HoldingAlly`) (<= (`self.GetDistanceTo` _weakguy self) 500.0))
      (`self.LaunchCharacter` _weakguy (+ (* (`SceneComponent.GetForwardVector` (`self.Camera`)) (`self.ChuckForce`)) (0.0 0.0 50.0)) false false)
      (`KismetSystemLibrary.PrintString` "Hello"))))

(fn `UserConstructionScript`
  (`parent.UserConstructionScript`))