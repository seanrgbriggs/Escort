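; Guardian is a Strong character Blueprint whose Attack2 input fires a chain power that pulls another player toward it.
; ChainPower sets a pull montage and runs a cone of line traces from the camera to find a PlayerBase.
; It launches that target toward the Guardian, adding upward lift that scales with distance.
; IsPulling blocks re-triggering until a short delay ends, but a non-PlayerBase hit never clears it.
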(event `self.ReceiveBeginPlay`
  (`parent.ReceiveBeginPlay`))

(event `self.ReceiveActorBeginOverlap`
  (params (OtherActor :type "Actor Object Reference")))

(event `self.ReceiveTick`
  (params (DeltaSeconds :type "Float (single-precision)"))
  (`parent.ReceiveTick` 0.0))

(event `InputAction|Attack2`
  (params (Key :type "Key Structure" :default "AnyKey"))
  (:`Pressed`
    (`self.ChainPower`)))

(event `ChainPower`
  (bind _camera (`self.Camera`))
  (if (not (`self.IsPulling`))
    (set `self.IsPulling` true)
    (set `self.PlayThisMontage` "/Game/Character/Animation/Strong/Guardian/strong_pull_montage.strong_pull_montage")
    (bind (_hit _success) (`self.ConeTraceLines` (`SceneComponent.K2_GetComponentLocation` _camera) (`SceneComponent.GetForwardVector` _camera) 2000.0 15.0 50.0 3 10))
    (if _success
      (bind _asplayer_base (cast `/Game/Character/Blueprints/PlayerBase` (`.HitActor` (`GameplayStatics.BreakHitResult` _hit))))
      (bind _returnvalue (- (`self.K2_GetActorLocation`) (`self.K2_GetActorLocation` _asplayer_base)))
      (`self.LaunchCharacter` _asplayer_base (* (+ (`KismetMathLibrary.Normal` _returnvalue) (`KismetMathLibrary.MakeVector` 0.0 0.0 (* (`KismetMathLibrary.VSize` _returnvalue) 0.0005))) (`self.PullStrength`)) true true))
    (`KismetSystemLibrary.Delay` 1.0)
    (set `self.IsPulling` false)))

(fn `UserConstructionScript`
  (`parent.UserConstructionScript`))