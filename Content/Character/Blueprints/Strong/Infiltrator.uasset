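; Infiltrator is a character Blueprint whose secondary attack spawns a decoy and hands the player control of it.
; Attack2 raycasts from the actor at 45 degrees downward along the camera's flattened forward direction to place an InfiltratorDecoy at the hit point.
; The decoy receives a parent reference and the same team, then the controller possesses it and the Infiltrator spawns a default controller for itself.
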(event `SpawnDecoy`
  (bind _returnvalue (`self.GetController`))
  (bind _camera (`self.Camera`))
  (bind (_hit _success) (`self.RaycastCall` 500.0 (`self.K2_GetActorLocation` self) (`KismetMathLibrary.RotateAngleAxis` (`KismetMathLibrary.ProjectVectorOnToPlane` (`SceneComponent.GetForwardVector` _camera) (0.0 0.0 1.0)) 45.0 (`SceneComponent.GetRightVector` _camera))))
  (if _success
    (bind _returnvalue_2 (`|SpawnActorFromClass` "/Game/Character/Blueprints/Weak/Infiltrator-Decoy.Infiltrator-Decoy_C" (`KismetMathLibrary.MakeTransform` (`.ImpactPoint` (`GameplayStatics.BreakHitResult` _hit)) (`KismetMathLibrary.Conv_VectorToRotator` (`SceneComponent.GetForwardVector` (`self.Camera`)))) "Undefined" "OverrideRootScale" _returnvalue))
    (set `/Game/Character/Blueprints/Weak/Infiltrator-Decoy.Parent` self _returnvalue_2)
    (`self.SetTeam` _returnvalue_2 (`self.Team`))
    (`Controller.Possess` _returnvalue _returnvalue_2)
    (`self.SpawnDefaultController`)))

(event `InputAction|Attack2`
  (params (Key :type "Key Structure" :default "AnyKey"))
  (:`Pressed`
    (`self.SpawnDecoy`)))

(fn `UserConstructionScript`
  (`parent.UserConstructionScript`))