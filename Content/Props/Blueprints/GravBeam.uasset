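; GravBeam is an actor that pulls overlapping Characters toward its center and lifts them upward.
; Every Tick it casts its overlapping actors to Character, then applies a swept offset toward its own location in X and Y, proportional to distance.
; It also calls LaunchCharacter with an additive, delta-time-scaled vertical velocity, so lift builds while overlap continues.
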(event `self.ReceiveBeginPlay`)

(event `self.ReceiveTick`
  (params (DeltaSeconds :type "Float (single-precision)"))
  (for _array_element (`self.GetOverlappingActors` null)
    (bind _ascharacter (cast `Character` _array_element))
    (`self.K2_AddActorWorldOffset` _ascharacter (`KismetMathLibrary.MakeVector` (.x (* (* (- (`self.K2_GetActorLocation`) (`self.K2_GetActorLocation` _ascharacter)) 3.0) DeltaSeconds)) (.y (* (* (- (`self.K2_GetActorLocation`) (`self.K2_GetActorLocation` _ascharacter)) 3.0) DeltaSeconds))) true false)
    (`Character.LaunchCharacter` _ascharacter (`KismetMathLibrary.MakeVector` 0.0 0.0 (* DeltaSeconds 2000.0)) false false)))

(fn `UserConstructionScript`)