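; Hurler projectile that damages and launches any player it hits.
; Hit forwards the hit target and location to ServerHit, which spawns an enlarged antimatter particle effect at that point.
; If the target is a PlayerBase, it is thrown along the projectile's forward direction with an upward boost and takes damage.
; The projectile then destroys itself, whatever it hit.
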(event `ServerHit`
  (params (OtherTarget :type "Actor Object Reference") (Loc :type "Vector Structure"))
  (bind _returnvalue (`GameplayStatics.SpawnEmitterAtLocation` "/Game/StarterContent/Particles/P_Antimatter.P_Antimatter" Loc))
  (`SceneComponent.SetWorldScale3D` _returnvalue (3.0 3.0 3.0))
  (bind _asplayer_base (cast `/Game/Character/Blueprints/PlayerBase` OtherTarget)
    (:`then`
      (`Character.LaunchCharacter` _asplayer_base (+ (* (`KismetMathLibrary.GetForwardVector` (`self.K2_GetActorRotation`)) 3000.0) (0.0 0.0 500.0)) false false)
      (`/Game/Character/Blueprints/PlayerBase.TakeDamage` _asplayer_base 100.0))
    (:`CastFailed`
      _))
  (`self.K2_DestroyActor`))

(event `self.ReceiveHit`
  (params (MyComp :type "PrimitiveComponent Object Reference") (Other :type "Actor Object Reference") (OtherComp :type "PrimitiveComponent Object Reference") (bSelfMoved :type Boolean) (HitLocation :type "Vector Structure") (HitNormal :type "Vector Structure") (NormalImpulse :type "Vector Structure") (Hit :type "HitResult Structure (by ref)"))
  (`self.ServerHit` Other HitLocation))

(fn `UserConstructionScript`)